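; BP_PlayerRogue is the player Blueprint that handles the UI responses to level-up and death.
; LevelUpSystem events open a card selection widget with near-frozen time dilation and UI-only input, then restore game input and normal speed once a card is picked.
; The HealthComponent death delegate clears all widgets, shows the game-over screen with a cursor, stops time dilation at zero and sets a short lifespan on the actor.
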(event OnLevelUpCardSelection(LevelUpSystem)
  (params (CardOptions :type Array%20of%20URF%20Card%20Option%20Structures))
  (bind _returnvalue (Game|GetPlayerController 0))
  ;[1 1 1] Card Level up System (Selection)
  (bind _returnvalue_2 (UserInterface|CreateWidget "/Game/URF_DemoA/Blueprints/HUD/WBP_CardWidget.WBP_CardWidget_C"))
  (UserInterface|Viewport|AddtoViewport _returnvalue_2 0)
  (Utilities|Time|SetGlobalTimeDilation 0.01)
  (Input|SetInputModeUIOnly _returnvalue _returnvalue_2 "DoNotLock")
  (Variables|/Script/Engine.PlayerController|SetbShowMouseCursor _returnvalue true))

(event OnCardSelected(LevelUpSystem)
  (params (SelectedCard :type URF%20Card%20Option%20Structure%20%28by%20ref%29))
  (bind _returnvalue (Game|GetPlayerController 0))
  ;[1 1 1] Card Level Up System (Selected)
  (Input|SetInputModeGameOnly _returnvalue)
  (Variables|/Script/Engine.PlayerController|SetbShowMouseCursor _returnvalue false)
  (Utilities|Time|SetGlobalTimeDilation 1.0))

(event OnDeathDelegate(HealthComponent)
  (params (Killer :type Actor%20Object%20Reference))
  ;[1 1 1] Death
  (Viewport|RemoveAllWidgets)
  (CallFunction|OpenGameOver)
  (Utilities|Time|SetGlobalTimeDilation 0.0)
  (Actor|SetLifeSpan 2.0))

(event Custom|OpenGameOver
  (Variables|/Script/Engine.PlayerController|SetbShowMouseCursor (Game|GetPlayerController 0) true)
  (bind _returnvalue (UserInterface|CreateWidget "/Game/URF_DemoA/Blueprints/HUD/WBP_GameOver.WBP_GameOver_C"))
  (UserInterface|Viewport|AddtoViewport _returnvalue 0))

(fn ConstructionScript)