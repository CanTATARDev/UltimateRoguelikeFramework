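; BP_Director is a wave-director Blueprint that reacts to wave, difficulty, time-limit and enemy-death events.
; On BeginPlay it binds handlers to those four delegates.
; The wave, difficulty and time-limit handlers only print colored debug messages, while the death handler stores the remaining enemy count.
; An unconnected "Boss Spawn" chain would stop wave management, slow time and destroy the player pawn after a short delay, but never runs.
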(event Custom|OnWaveStartedDelegate_Event
  (params (WaveNumber :type Integer) (WaveTemplate :type URF%20Wave%20Template%20Structure%20%28by%20ref%29))
  (Development|PrintString "Wave Started" true true "(R=1.000000,G=0.000000,B=0.141900,A=1.000000)"))

(event Custom|OnTimeLimitReachedDelegate_Event
  (params (TotalGameTime :type Float%20%28single-precision%29))
  (Development|PrintString "GameTime Finish" true true "(R=0.000000,G=0.490066,B=1.000000,A=1.000000)" 1e+01))

(event Custom|OnDifficultyChangedDelegate_Event
  (params (NewDifficulty :type Float%20%28single-precision%29))
  (Development|PrintString "Hard++" true true "(R=0.000000,G=1.000000,B=0.673462,A=1.000000)"))

(event Custom|CustomEvent_0
  (params (Enemy :type Actor%20Object%20Reference) (RemainingEnemies :type Integer))
  (Variables|Default|SetRemaining%20Enemies RemainingEnemies))

(event EventBeginPlay
  (EventDispatchers|BindEventtoOnWaveStartedDelegate (delegate Custom|OnWaveStartedDelegate_Event))
  (EventDispatchers|BindEventtoOnDifficultyChangedDelegate (delegate Custom|OnDifficultyChangedDelegate_Event))
  (EventDispatchers|BindEventtoOnTimeLimitReachedDelegate (delegate Custom|OnTimeLimitReachedDelegate_Event))
  (EventDispatchers|BindEventtoOnEnemyDiedDelegate (delegate Custom|CustomEvent_0)))

(fn ConstructionScript)