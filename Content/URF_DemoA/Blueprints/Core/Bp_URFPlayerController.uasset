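; Player controller for the URF demo that opens an in-game settings menu on Tab and pauses the game.
; Tab creates the WBP_SettingsMenu widget and adds it to the viewport on first use, then makes the stored instance visible on later presses.
; PauseGame pauses the game, shows the mouse cursor and switches input to Game and UI with focus on the menu.
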(event Custom|PauseGame
  (Game|SetGamePaused true)
  (Variables|Default|SetbShowMouseCursor true)
  (Input|SetInputModeGameandUI self (Variables|Default|GetSettingsMenuUI) "DoNotLock" true))

(event Input|KeyboardEvents|Tab
  (params (Key :type Key%20Structure :default "None"))
  (:Pressed
    (bind _settingsmenuui (Variables|Default|GetSettingsMenuUI)
      (:then
        (Widget|SetVisibility _settingsmenuui "Visible")
        (CallFunction|PauseGame))
      (:else
        (bind _returnvalue (UserInterface|CreateWidget "/Game/URF_DemoA/Blueprints/HUD/WBP_SettingsMenu.WBP_SettingsMenu_C" self))
        (Variables|Default|SetSettingsMenuUI _returnvalue)
        (UserInterface|Viewport|AddtoViewport (Variables|Default|GetSettingsMenuUI) 0)
        (CallFunction|PauseGame)))))

(fn ConstructionScript)